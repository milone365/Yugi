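; Game manager Blueprint for a card battle between the player and a computer opponent.
; On BeginPlay it links to the player controller and screen, copies the DeckBp deck and finds the FusionController.
; PlayCard has the FusionController pick from five random enemy draws, then trades Atk-minus-Def damage both ways and clears the table.
; Enemy defeat shows the game clear widget, and LoseGame shows game over.
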(event Custom|PlayCard
  (params (NewParam :type Card%20Data%20Structure))
  (if (Variables|Default|GetCombatPhase)
    (Variables|Default|SetCombatPhase false)
    (CallFunction|SelectEnemyCard)
    (Default|PlayBattle (Variables|/Game/PlayerControllerBP.PlayerControllerBP_C|GetScreen (Variables|Default|GetPlayer)))
    (Utilities|FlowControl|Delay 3.0)
    (CallFunction|Battle NewParam (Variables|Default|GetEnemyCard))))

(event Custom|ClearTable
  (bind _player (Variables|Default|GetPlayer))
  (bind _screen (Variables|/Game/PlayerControllerBP.PlayerControllerBP_C|GetScreen _player))
  (Utilities|FlowControl|Delay 2.0)
  (Default|BattleOff _screen)
  (Utilities|FlowControl|Delay 2.0)
  (Variables|/Game/UI/GameWidget.GameWidget_C|SetSelectedCard _screen (Utilities|Struct|MakeCardData "" 0 0 0 "(Material1_2_37D875EC41352E75C1EE4F9B0680B03C=\"\",Material2_4_A93555E8470A8710F47F848852566D8F=\"\")" false))
  (Variables|Default|SetCombatPhase true))

(event EventBeginPlay
  (bind _self self)
  ;[1 1 1] START
  (Utilities|FlowControl|Delay 3.0)
  (bind _returnvalue (Actor|GetActorOfClass "/Game/PlayerControllerBP.PlayerControllerBP_C"))
  (Variables|Default|SetPlayer _returnvalue)
  (Variables|/Game/UI/GameWidget.GameWidget_C|SetGameManager (Variables|/Game/PlayerControllerBP.PlayerControllerBP_C|GetScreen (Variables|Default|GetPlayer)) _self)
  (Default|SetGM (Variables|Default|GetPlayer) _self)
  (CallFunction|BuildEnemyDeck)
  (bind _returnvalue_2 (Actor|GetActorOfClass "/Game/FusionController.FusionController_C"))
  (Variables|Default|SetFusionController _returnvalue_2)
  (Variables|Default|SetCombatPhase true))

(fn ConstructionScript)

(fn Battle
  (params (PlayerCard :type Card%20Data%20Structure) (EnemyCard :type Card%20Data%20Structure))
  (bind (_name _atk _def) (Utilities|Struct|BreakCardData PlayerCard))
  (bind (_name_2 _atk_2 _def_2) (Utilities|Struct|BreakCardData EnemyCard))
  (bind _newparam2 (CallFunction|GetDamage _atk_2 _def))
  (Default|TakeDamage (Variables|Default|GetPlayer) _newparam2)
  (bind _newparam2_2 (CallFunction|GetDamage _atk _def_2))
  (CallFunction|PcTakeDamage _newparam2_2)
  (CallFunction|ClearTable))

(fn SelectEnemyCard
  (bind _hand (CallFunction|GetHand))
  (bind _cardtoplay (Default|PcPlayCard (Variables|Default|GetFusionController) _hand))
  (Variables|Default|SetEnemyCard _cardtoplay))

(fn GetDamage
  (params (Atk :type Integer) (Def :type Integer))
  (bind _returnvalue (- Atk Def))
  (if (<= _returnvalue 0)
    (LocalVariables|Setlocaldamage 0)
    (else
      (LocalVariables|Setlocaldamage _returnvalue)))
  (return (LocalVariables|Getlocaldamage)))

(fn LoseGame
  (bind _returnvalue (UserInterface|CreateWidget "/Game/UI/GameOverWidget.GameOverWidget_C"))
  (UserInterface|Viewport|AddtoViewport _returnvalue 0))

(fn GameEnd
  (bind _returnvalue (UserInterface|CreateWidget "/Game/UI/GameClearWidget.GameClearWidget_C"))
  (UserInterface|Viewport|AddtoViewport _returnvalue 0))

(fn PcTakeDamage
  (params (NewParam :type Integer))
  (bind _output_get (Variables|Default|SetEnemyHp (- (Variables|Default|GetEnemyHp) NewParam)))
  (if (<= _output_get 0)
    (CallFunction|GameEnd)))

(fn BuildEnemyDeck
  (bind _returnvalue (Actor|GetActorOfClass "/Game/DATA/DeckBp.DeckBp_C"))
  (Utilities|IsValid _returnvalue
    (:Is%20Valid
      (for _array_element (Variables|/Game/DATA/DeckBp.DeckBp_C|GetDeck _returnvalue)
        (Utilities|Array|Add (Variables|Default|GetEnemyDeck) _array_element)))))

(fn GetHand
  (bind _enemydeck (Variables|Default|GetEnemyDeck))
  (for _index (range 1 5)
    (Utilities|Array|Add (LocalVariables|GetTemp_Hand) (Utilities|Array|Get(acopy) _enemydeck (Math|Random|RandomIntegerinRange 0 (- (Utilities|Array|Length _enemydeck) 1)))))
  (return (LocalVariables|GetTemp_Hand)))