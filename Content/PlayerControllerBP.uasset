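; Player controller for a card game with card fusion, holding the player's hand, HP and combo points.
; After a short startup delay it finds the player deck, draws an opening hand, creates the game HUD and caches the FusionController.
; Played cards are replaced from the deck; if absent from the hand, their two fusion materials are replaced instead.
; Capped combo points set the healing amount, and depleted HP tells the game manager to lose.
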(event Custom|AddComboPoint
  ;[1 1 1] ADDCOMBO
  (if (> (+ (Variables|Default|GetComboPoint) 1) 5)
    (Variables|Default|SetComboPoint 5)
    (else
      (Variables|Default|SetComboPoint (+ (Variables|Default|GetComboPoint) 1)))))

(event Custom|ClearCombo
  (Variables|Default|SetComboPoint 0))

(event EventBeginPlay
  (Utilities|FlowControl|Delay 2.0)
  (bind _outactors (Actor|GetAllActorsOfClass "/Game/DATA/DeckBp.DeckBp_C"))
  (for _array_element _outactors
    (if (Variables|/Game/DATA/DeckBp.DeckBp_C|GetPlayerdeck _array_element)
      (Variables|Default|SetDeck _array_element)
      (for _index (range 1 5)
        (CallFunction|DrawCard))
      (bind _returnvalue (UserInterface|CreateWidget "/Game/UI/GameWidget.GameWidget_C"))
      (bind _output_get (Variables|Default|SetScreen _returnvalue))
      (UserInterface|Viewport|AddtoViewport _output_get 0)
      (Variables|/Game/UI/GameWidget.GameWidget_C|SetPlayer (Variables|Default|GetScreen) self)
      (bind _returnvalue_2 (Actor|GetActorOfClass "/Game/FusionController.FusionController_C"))
      (Variables|Default|SetFusionController _returnvalue_2)
      (Default|SetElement (Variables|Default|GetScreen) (Variables|Default|GetElement) true))))

(fn ConstructionScript)

(fn DrawCard
  (Utilities|FlowControl|Sequence
    (:then_0
      (bind (_array_element _array_index) (Utilities|Array|ForEachLoopwithBreak (Variables|Default|GetHand) :!label _label)
        (:LoopBody
          (if (Utilities|Enum|Equal(Enum) (.Name (Utilities|Struct|BreakCardData _array_element)) "")
            (LocalVariables|Setindex _array_index)
            (goto _label Break)))))
    (:then_1
      (bind _newparam (Default|DrawCard (Variables|Default|GetDeck)))
      (Utilities|Array|SetArrayElem (Variables|Default|GetHand) (LocalVariables|Getindex) _newparam))))

(fn TakeDamage
  (params (NewParam :type Integer))
  (bind _output_get (Variables|Default|SetHP (- (Variables|Default|GetHP) NewParam)))
  (if (<= _output_get 0)
    (Default|LoseGame (Variables|Default|GetGamemanager))))

(fn SetGM
  (params (NewParam :type Game%20Manager%20BP%20Object%20Reference))
  (Variables|Default|SetGamemanager NewParam))

(fn ClearHand
  (params (playedCard :type Card%20Data%20Structure))
  (bind _found (CallFunction|ClearCard (.Name (Utilities|Struct|BreakCardData playedCard))))
  (if _found
    (CallFunction|DrawCard)
    (else
      (bind (_m1 _m2) (Default|GetMaterials (Variables|Default|GetFusionController) playedCard))
      (CallFunction|ClearCard _m1)
      (CallFunction|ClearCard _m2)
      (CallFunction|DrawCard)
      (CallFunction|DrawCard))))

(fn ClearCard
  (params (NewParam :type String))
  (Utilities|FlowControl|Sequence
    (:then_0
      (bind (_array_element _array_index) (Utilities|Array|ForEachLoopwithBreak (Variables|Default|GetHand) :!label _label)
        (:LoopBody
          (bind _output_get (LocalVariables|SetFounded (Utilities|Enum|Equal(Enum) NewParam (.Name (Utilities|Struct|BreakCardData _array_element)))))
          (if _output_get
            (LocalVariables|Setindex _array_index)
            (goto _label Break)))))
    (:then_1
      (if (LocalVariables|GetFounded)
        (Utilities|Array|SetArrayElem (Variables|Default|GetHand) (LocalVariables|Getindex) (Utilities|Struct|MakeCardData "" 0 0 0 "(Material1_2_37D875EC41352E75C1EE4F9B0680B03C=\"\",Material2_4_A93555E8470A8710F47F848852566D8F=\"\")" false))))
    (:then_2
      (return (LocalVariables|GetFounded)))))

(fn Healing
  (Variables|Default|SetHP (+ (Variables|Default|GetHP) (Variables|Default|GetComboPoint))))