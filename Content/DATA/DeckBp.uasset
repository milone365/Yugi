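; Card deck Blueprint that builds a deck from the CardList data table and hands out random cards.
; On BeginPlay it adds three copies of each row to Deck, with a parallel DrawedCards bool array starting false.
; DrawCard flags a random index as drawn, then returns a card from a separately rolled index, without checking the flags.
; Both rolls use the array length as inclusive maximum, so can land out of range.
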(event EventBeginPlay
  ;[1 1 1] BuildDeck
  (bind _outrownames (DataTable|GetDataTableRowNames (Variables|Default|GetcardList)))
  (for _array_element _outrownames
    (bind _returnvalue (Utilities|GetDataTableRow (Variables|Default|GetcardList) _array_element)
      (:then
        (for _index (range 1 3)
          (Utilities|Array|Add (Variables|Default|GetDeck) _returnvalue)
          (Utilities|Array|Add (Variables|Default|GetDrawedCards) false))))))

(fn ConstructionScript)

(fn DrawCard
  (bind _deck (Variables|Default|GetDeck))
  (bind _returnvalue (Utilities|Array|Length _deck))
  (bind _returnvalue_2 (Math|Random|RandomIntegerinRange 0 _returnvalue))
  (while (not (LocalVariables|GetIsEqual))
    (Utilities|Array|SetArrayElem (Variables|Default|GetDrawedCards) _returnvalue_2 true)
    (LocalVariables|SetIsEqual true))
  (return (Utilities|Array|Get(acopy) (Variables|Default|GetDeck) _returnvalue_2)))